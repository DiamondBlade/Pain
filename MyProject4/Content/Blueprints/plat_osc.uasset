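; Oscillating platform actor that moves its PlatformBase component back and forth between the Start and End component locations.
; Each tick it maps a sine of game time, divided by TimeScaleInverse, into a 0–1 alpha and interpolates between the two world positions.
; Because motion derives from absolute game time, it keeps no state, and the location is set without sweeping for collisions.
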(event EventBeginPlay)

(event Collision|EventActorBeginOverlap
  (params (OtherActor :type Actor%20Object%20Reference)))

(event EventTick
  (params (DeltaSeconds :type Float%20%28single-precision%29))
  (Transformation|SetWorldLocation (Variables|Default|GetplatformBase) (.location (Math|Transform|Lerp(Transform) (Math|Transform|MakeTransform (Transformation|GetWorldLocation (Variables|Default|GetStart)) "0, 0, 0" "1,1,1") (Math|Transform|MakeTransform (Transformation|GetWorldLocation (Variables|Default|GetEnd)) "0, 0, 0" "1,1,1") (/ (+ (Math|Trig|Sin(Radians) (/ (Utilities|Time|GetGameTimeinSeconds) (Variables|Default|GetTimeScaleInverse))) 1.0) 2.0))) false false))

(fn ConstructionScript)